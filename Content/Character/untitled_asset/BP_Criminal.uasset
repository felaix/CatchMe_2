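; BP_Criminal is the player character, who interacts with objects and can be found and killed.
; InteractBox overlaps with Interface_Interact actors toggle a prompt widget and let the Interact input send InteractMessage to the overlapped actor.
; A "Kill"-tagged component entering Box triggers Kill, which flags the anim instance, disables input and ragdolls the mesh.
; After a short delay it destroys the actor, then calls PlayerWasFound on BP_TopDownGameMode.
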(event OnComponentEndOverlap(interactBox)
  (params (OverlappedComponent :type Primitive%20Component%20Object%20Reference) (OtherActor :type Actor%20Object%20Reference) (OtherComp :type Primitive%20Component%20Object%20Reference) (OtherBodyIndex :type Integer))
  ;[1 0.9604 0.1499] Check if interactable in front of player
  (if (Utilities|DoesObjectImplementInterface OtherActor "/Game/Blueprints/Interfaces/Interface_Interact.Interface_Interact_C")
    (Variables|Default|SetbInteractable false)
    (CallFunction|InteractUI false)))

(event OnComponentBeginOverlap(interactBox)
  (params (OverlappedComponent :type Primitive%20Component%20Object%20Reference) (OtherActor :type Actor%20Object%20Reference) (OtherComp :type Primitive%20Component%20Object%20Reference) (OtherBodyIndex :type Integer) (bFromSweep :type Boolean) (SweepResult :type Hit%20Result%20Structure%20%28by%20ref%29))
  ;[1 0.9604 0.1499] Check if interactable in front of player
  (if (Utilities|DoesObjectImplementInterface OtherActor "/Game/Blueprints/Interfaces/Interface_Interact.Interface_Interact_C")
    (Variables|Default|SetbInteractable true)
    (CallFunction|InteractUI true)))

(event OnComponentBeginOverlap(Box)
  (params (OverlappedComponent :type Primitive%20Component%20Object%20Reference) (OtherActor :type Actor%20Object%20Reference) (OtherComp :type Primitive%20Component%20Object%20Reference) (OtherBodyIndex :type Integer) (bFromSweep :type Boolean) (SweepResult :type Hit%20Result%20Structure%20%28by%20ref%29))
  ;[1 0 0] Trigger KIll
  (if (Components|ComponentHasTag OtherComp "Kill")
    (CallFunction|Kill)))

(event Custom|InteractUI
  (params (Show :type Boolean))
  ;[0.4072 0.3763 0] Show Interact UI
  (if Show
    (if (not (Variables|Default|GetbInteractUI))
      (bind _returnvalue (UserInterface|CreateWidget "/Game/UI/UI_Interact.UI_Interact_C"))
      (UserInterface|Viewport|AddtoViewport _returnvalue 0)
      (Variables|Default|SetbInteractUI true))
    (elif (Variables|Default|GetbInteractUI)
      (Widget|RemovefromParent _returnvalue)
      (Variables|Default|SetbInteractUI false))))

(event Custom|Kill
  ;[1 0 0] Kill
  (bind _asabp_criminal (Utilities|Casting|CastToABP_Criminal (Components|SkeletalMesh|GetAnimInstance (Variables|Character|GetMesh))))
  (Variables|/Game/Character/untitled_asset/ABP_Criminal.ABP_Criminal_C|SetisFound _asabp_criminal true)
  (Input|DisableInput self (Game|GetPlayerController 0))
  (Collision|SetCollisionEnabled (Variables|Collision|GetCapsuleComponent) "NoCollision")
  (Pawn|Components|CharacterMovement|SetMovementMode (Variables|Character|GetCharacterMovement) "MOVE_None" 0)
  (Physics|SetSimulatePhysics (Variables|Character|GetMesh) true)
  (Collision|SetCollisionProfileName (Variables|Character|GetMesh) "Ragdoll" true :!class /Script/Engine.PrimitiveComponent)
  (Utilities|FlowControl|Delay 1.0)
  (Actor|DestroyActor)
  (bind _asbp_top_down_game_mode (Utilities|Casting|CastToBP_TopDownGameMode (Game|GetGameMode)))
  (Default|PlayerWasFound _asbp_top_down_game_mode))

(event EventBeginPlay
  ;[0 0 0] Create UI
  (bind _returnvalue (UserInterface|CreateWidget "/Game/UI/UI_Main.UI_Main_C"))
  (UserInterface|Viewport|AddtoViewport _returnvalue 0))

(event Input|ActionEvents|InputActionInteract
  (params (Key :type Key%20Structure :default "None"))
  ;[1 0.9216 0] Interact
  (:Pressed
    (if (Variables|Default|GetbInteractable)
      (Class|InterfaceInteract|Interact(Message) (stale OnComponentBeginOverlap(interactBox) OtherActor))
      (else
        (Development|PrintString "Not interactable" true true "(R=1.000000,G=0.033346,B=0.000000,A=1.000000)")))
    (CallFunction|InteractUI false)))

(fn ConstructionScript)