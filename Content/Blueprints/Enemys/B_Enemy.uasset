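; Enemy actor that patrols along a referenced spline actor and detects the player through a collision component.
; On BeginPlay a timeline, with play rate set to the inverse of Speed, lerps distance over the spline's length to set location and rotation.
; Location is sampled in world space and rotation in local space.
; Overlaps with components tagged "player" only print a red debug message.
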(event OnComponentBeginOverlap(Col_detection)
  (params (OverlappedComponent :type Primitive%20Component%20Object%20Reference) (OtherActor :type Actor%20Object%20Reference) (OtherComp :type Primitive%20Component%20Object%20Reference) (OtherBodyIndex :type Integer) (bFromSweep :type Boolean) (SweepResult :type Hit%20Result%20Structure%20%28by%20ref%29))
  (if (Components|ComponentHasTag OtherComp "player")
    (Development|PrintString "PLAYER DETECTED" true true "(R=1.000000,G=0.000000,B=0.009271,A=1.000000)")))

(event Custom|FollowSpline
  (bind _refspline (Variables|Default|GetrefSpline))
  (bind _spline (Variables|/Game/Blueprints/Enemys/B_Spline.B_Spline_C|GetSpline _refspline))
  (Components|Timeline|SetPlayRate (Variables|Default|GetT_Move) (/ 1.0 (Variables|Default|GetSpeed)))
  (bind _value (Timeline|T_Move Play)
    (:Update
      (Transformation|SetActorTransform (Math|Transform|MakeTransform (Spline|GetLocationatDistanceAlongSpline _spline (Math|Float|Lerp 0.0 (Spline|GetSplineLength _spline) _value) "World") (Spline|GetRotationatDistanceAlongSpline _spline (Math|Float|Lerp 0.0 (Spline|GetSplineLength _spline) _value) "Local") "1.000000,1.000000,1.000000")))))

(event EventBeginPlay
  (CallFunction|FollowSpline))

(fn ConstructionScript)