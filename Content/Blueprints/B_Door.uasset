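; B_Door is an interactable door that opens a new area once the player has collected the required items.
; On Interact it asks the cached BP_TopDownGameMode to check the B_Item class, then reads its AllCollected flag.
; It shows a UI_Message widget with either the new-area text, destroying itself after a short delay, or the text saying what is still needed.
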(event EventInteract
  (bind _gamemode (Variables|Default|GetGameMode))
  (Default|CheckClass _gamemode "/Game/Blueprints/B_Item.B_Item_C")
  (if (Variables|/Game/TopDown/Blueprints/BP_TopDownGameMode.BP_TopDownGameMode_C|GetallCollected _gamemode)
    (bind _returnvalue (UserInterface|CreateWidget "/Game/UI/UI_Message.UI_Message_C"))
    (UserInterface|Viewport|AddtoViewport _returnvalue 0)
    (Default|ChangeText _returnvalue (Variables|Default|GetnewAreaText))
    (Utilities|FlowControl|Delay 0.2)
    (Actor|DestroyActor)
    (else
      (bind _returnvalue_2 (UserInterface|CreateWidget "/Game/UI/UI_Message.UI_Message_C"))
      (UserInterface|Viewport|AddtoViewport _returnvalue_2 0)
      (Default|ChangeText _returnvalue_2 (Variables|Default|GetNeedText)))))

(event EventBeginPlay
  (bind _returnvalue (Actor|GetActorOfClass "/Game/TopDown/Blueprints/BP_TopDownGameMode.BP_TopDownGameMode_C"))
  (Variables|Default|SetGameMode _returnvalue))

(fn ConstructionScript)