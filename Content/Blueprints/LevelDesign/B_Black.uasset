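; B_Black is a level-design trigger actor that announces a newly unlocked area and then removes itself.
; When a component tagged "player" overlaps its Box, it prints a debug string and runs activateArea.
; That event shows a UI_Message widget with the UnlockMessage text, then destroys the actor after a short delay.
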(event OnComponentBeginOverlap(Box)
  (params (OverlappedComponent :type Primitive%20Component%20Object%20Reference) (OtherActor :type Actor%20Object%20Reference) (OtherComp :type Primitive%20Component%20Object%20Reference) (OtherBodyIndex :type Integer) (bFromSweep :type Boolean) (SweepResult :type Hit%20Result%20Structure%20%28by%20ref%29))
  (if (Components|ComponentHasTag OtherComp "player")
    (Development|PrintString "NEW AREA")
    (CallFunction|ActivateArea)))

(event Custom|activateArea
  (bind _returnvalue (UserInterface|CreateWidget "/Game/UI/UI_Message.UI_Message_C"))
  (UserInterface|Viewport|AddtoViewport _returnvalue 0)
  (Default|ChangeText _returnvalue (Variables|Default|GetUnlockMessage))
  (Utilities|FlowControl|Delay 0.1)
  (Actor|DestroyActor))

(event EventBeginPlay)

(event Collision|EventActorBeginOverlap
  (params (OtherActor :type Actor%20Object%20Reference)))

(event EventTick
  (params (DeltaSeconds :type Float%20%28single-precision%29)))

(fn ConstructionScript)