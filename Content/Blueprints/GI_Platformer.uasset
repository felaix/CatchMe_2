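; GI_Platformer is the platformer's game instance blueprint that manages background music across level transitions.
; ChangeBackgroundMusic creates a persistent 2D audio component on first use and stores it for reuse.
; Later changes stop that component with a zero-length fade, wait briefly, swap the sound and restart it.
; AdjustBackgroundMusicVolume linearly moves the same component's volume to a given level over a given duration.
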(event Custom|Change%20Background%20Music
  (params (New%20Background%20Music :type Sound%20Base%20Object%20Reference))
  (Variables|Default|GetBackgroundMusicComponent
    (:then
      (Audio|Components|Audio|FadeOut (Variables|Default|GetBackgroundMusicComponent) 0.0 0.0 "Linear" :!class /Script/Engine.AudioComponent)
      (Utilities|FlowControl|Delay 1.0)
      (Audio|Components|Audio|SetSound (Variables|Default|GetBackgroundMusicComponent) New%20Background%20Music))
    (:else
      (bind _returnvalue (Audio|CreateSound2D New%20Background%20Music 1.0 1.0 0.0 0 true))
      (Variables|Default|SetBackgroundMusicComponent _returnvalue)))
  (Audio|Components|Audio|Play (Variables|Default|GetBackgroundMusicComponent) 0.0)
  (Audio|Components|Audio|FadeIn (Variables|Default|GetBackgroundMusicComponent) 0.0 1.0 0.0 "Linear" :!class /Script/Engine.AudioComponent))

(event Custom|Adjust%20Background%20Music%20Volume
  (params (AdjustVolumeDuration :type Float%20%28double-precision%29) (AdjustVolumeLevel :type Float%20%28double-precision%29))
  (Audio|Components|Audio|AdjustVolume (Variables|Default|GetBackgroundMusicComponent) AdjustVolumeDuration AdjustVolumeLevel "Linear" :!class /Script/Engine.AudioComponent))